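; Projectile fired by BP_Tank, taking its initial speed from the instigating tank's LaunchSpeed in the construction script.
; BeginPlay caches a Landscape reference for render-target painting.
; An unconnected chain would trace down on movement and draw M_Quad into T_RenderTo at the landscape-relative hit position, sized by HoleScale.
; That drawing logic never runs, as Tick is empty.
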(event Collision|EventActorBeginOverlap
  (params (OtherActor :type Actor%20Object%20Reference)))

(event EventTick
  (params (DeltaSeconds :type Float%20%28single-precision%29)))

(event EventBeginPlay
  ;[0.2969 0.2969 0.2969] Deal with rendertarget & landscape ref
  (bind _outactors (Actor|GetAllActorsOfClass "/Script/Landscape.Landscape"))
  (for _array_element _outactors
    (Variables|Default|SetLandscape _array_element)))

(fn ConstructionScript
  (bind _asbp_tank (Utilities|Casting|CastToBP_Tank (Game|GetInstigator)))
  (Variables|/Script/Engine.ProjectileMovementComponent|SetInitialSpeed (Variables|Default|GetProjectileMovement) (Variables|/Script/BattleTank.Tank|GetLaunchSpeed _asbp_tank)))